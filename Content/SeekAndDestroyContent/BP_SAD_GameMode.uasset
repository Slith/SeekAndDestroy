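; Game mode for the SAD (Seek and Destroy) game that connects game phase changes to the UI and player input.
; On BeginPlay it binds to phase changes, takes the configuration and HUD widgets from its widget components, and adds both to the viewport before calling the parent.
; Each phase change is forwarded to both widgets and sets input mode and cursor: UI-only for Configuration and End, game-only for Play.
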(event EventBeginPlay
  (EventDispatchers|AssignGamePhaseChanging (EventDispatchers|CreateEvent :!event OnGamePhaseChanging))
  (bind _output_get (Variables|Default|SetWidgetGameConfiguration (.AsWBP%20SAD%20Game%20Configuration (Utilities|Casting|CastToWBP_SAD_GameConfiguration (UserInterface|GetWidget (Variables|Default|GetWC_GameConfiguration))))))
  (bind _output_get_2 (Variables|Default|SetWidgetHUD (.AsWBP%20SAD%20Game%20HUD (Utilities|Casting|CastToWBP_SAD_GameHUD (UserInterface|GetWidget (Variables|Default|GetWC_HUD))))))
  (UserInterface|Viewport|AddtoViewport _output_get 0)
  (|CallParentFunction))

(fn ConstructionScript)

(fn OnGamePhaseChanging
  (params (NewGamePhase :type EGamePhase%20Enum :default "Configuration"))
  (CallFunction|UpdateInputMode NewGamePhase)
  (Default|OnGamePhaseChanging (Variables|Default|GetWidgetGameConfiguration) NewGamePhase)
  (Default|OnGamePhaseChanging (Variables|Default|GetWidgetHUD) NewGamePhase))

(fn UpdateInputMode
  (params (NewGamePhase :type EGamePhase%20Enum :default "Configuration"))
  (bind _returnvalue (Game|GetPlayerController 0))
  (switch Utilities|FlowControl|Switch|SwitchonEGamePhase NewGamePhase
    (:Configuration
      (Input|SetInputModeUIOnly _returnvalue (Variables|Default|GetWidgetGameConfiguration) "DoNotLock")
      (Variables|/Script/Engine.PlayerController|SetbShowMouseCursor _returnvalue true))
    (:Play
      (Input|SetInputModeGameOnly _returnvalue)
      (Variables|/Script/Engine.PlayerController|SetbShowMouseCursor _returnvalue false))
    (:End
      (Input|SetInputModeUIOnly _returnvalue (Variables|Default|GetWidgetHUD) "DoNotLock")
      (Variables|/Script/Engine.PlayerController|SetbShowMouseCursor _returnvalue true))))