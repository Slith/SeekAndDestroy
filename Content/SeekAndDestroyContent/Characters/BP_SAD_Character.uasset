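; BP_SAD_Character is a Seek and Destroy character Blueprint that keeps a status widget in sync with the character's health.
; On BeginPlay it caches WBP_CharacterStatus from the WCStatus widget component, sets initial values and binds to health and max health change events.
; UpdateWidgetStatus pushes both values to the widget, playing the hit animation only when triggered by AnyDamage.
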(event Custom|HealthChanged_Event
  (params (NewValue :type Float%20%28single-precision%29))
  (CallFunction|UpdateWidgetStatus false))

(event Custom|MaxHealthChanged_Event
  (params (NewValue :type Float%20%28single-precision%29))
  (CallFunction|UpdateWidgetStatus false))

(event EventBeginPlay
  (Variables|Default|SetWidgetStatus (.AsWBP%20Character%20Status (Utilities|Casting|CastToWBP_CharacterStatus (UserInterface|GetWidget (Variables|Default|GetWC_Status)))))
  (CallFunction|UpdateWidgetStatus false)
  (EventDispatchers|AssignHealthChanged (delegate Custom|HealthChanged_Event))
  (EventDispatchers|AssignMaxHealthChanged (delegate Custom|MaxHealthChanged_Event)))

(event Game|Damage|EventAnyDamage
  (params (Damage :type Float%20%28single-precision%29) (DamageType :type Damage%20Type%20Object%20Reference) (InstigatedBy :type Controller%20Object%20Reference) (DamageCauser :type Actor%20Object%20Reference))
  (CallFunction|UpdateWidgetStatus true))

(fn ConstructionScript)

(fn UpdateWidgetStatus
  (params (PlayHitAnimation :type Boolean))
  (Default|SetHealth (Variables|Default|GetWidgetStatus) (Class|SeekandDestroyCharacter|GetHealth) (Class|SeekandDestroyCharacter|GetMaxHealth) PlayHitAnimation))