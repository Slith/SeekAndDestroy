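; BP_SAD_PlayerCharacter is the player character Blueprint for Seek and Destroy, which starts play armed with a default gun.
; On BeginPlay it spawns a BP_SAD_DefaultGun at its own transform with itself as instigator, then equips it through EquipWeapon.
; The held weapon is then snap-attached to the right index finger socket on the character mesh.
; Construction only calls the parent script.
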(event EventBeginPlay
  (|CallParentFunction)
  (bind _returnvalue (Game|SpawnActorfromClass "/Game/SeekAndDestroyContent/Weapons/BP_SAD_DefaultGun.BP_SAD_DefaultGun_C" (Math|Transform|MakeTransform (Transformation|GetActorLocation) (Transformation|GetActorRotation)) "AlwaysSpawn" 0 self))
  (Class|SeekandDestroyCharacter|EquipWeapon _returnvalue)
  (Transformation|AttachComponentToComponent (Class|SeekandDestroyCharacter|GetHeldWeapon) (Variables|Character|GetMesh) "index_02_r" "SnapToTarget" "SnapToTarget" "SnapToTarget" true))

(fn ConstructionScript
  (|CallParentFunction))